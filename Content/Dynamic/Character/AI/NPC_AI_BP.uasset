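; AI controller for NPC guards that starts the GuardBehaviour tree with the PatrolData blackboard.
; Perception writes sensed actors lacking the "Enemy" tag to the blackboard's enemy key and clears the key when sensing fails.
; Every tick, it sets the pawn's Aiming and Shooting flags according to whether the controller has a valid focus actor.
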(event `self.ReceiveBeginPlay`
  (bind _blackboardcomponent (`self.UseBlackboard` "/Game/Dynamic/Character/AI/PatrolData.PatrolData"))
  (`self.RunBehaviorTree` "/Game/Dynamic/Character/AI/GuardBehaviour.GuardBehaviour")
  (set `self.Blackboard Component` _blackboardcomponent))

(event `self.ReceiveTick`
  (params (DeltaSeconds :type "Float (single-precision)"))
  (bind _returnvalue (`KismetSystemLibrary.IsValid` (`self.GetFocusActor`)))
  (bind _astpcharacter (cast `/Game/Dynamic/Character/Behaviour/Character` (`self.K2_GetPawn`)))
  (set `/Game/Dynamic/Character/Behaviour/Character.Aiming` _returnvalue _astpcharacter)
  (set `/Game/Dynamic/Character/Behaviour/Character.Shooting` _returnvalue _astpcharacter))

(event `self.AIPerception.OnTargetPerceptionUpdated`
  (params (Actor :type "Actor Object Reference") (Stimulus :type "AIStimulus Structure"))
  (bind _blackboard_component (`self.Blackboard Component`))
  (bind _enemykey (`self.EnemyKey`))
  (if (`self.ActorHasTag` Actor "Enemy")
    _
    (elif (`.bSuccessfullySensed` (break `AIStimulus` Stimulus))
      (`BlackboardComponent.SetValueAsObject` _blackboard_component _enemykey Actor)
      (else
        (`BlackboardComponent.ClearValue` _blackboard_component _enemykey)))))

(fn `UserConstructionScript`)